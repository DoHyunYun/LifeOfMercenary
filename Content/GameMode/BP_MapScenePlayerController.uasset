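; Player controller for the map scene that pans the view by moving the player pawn with touch drags.
; On BeginPlay it creates the UI_MapPoint widget, registers it with the HUD manager and activates the touch interface.
; Touch movement at least Sensitivity away from the press point sets IsTouchMove and offsets the pawn by the inverted drag delta, rotated 90 degrees and scaled by Power.
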(event `self.ReceiveBeginPlay`
  (bind _returnvalue (`|CreateWidget` "/Game/UI/UI_MapPoint.UI_MapPoint_C" null null))
  (`UserWidget.AddToViewport` _returnvalue 0)
  (bind _returnvalue_2 (`LoMFunctions.GetHUDManager`))
  (`HUDManager.AddUI` _returnvalue_2 _returnvalue "UI_MapPoint")
  (`self.ActivateTouchInterface` null))

(event `InputTouch`
  (params (Location :type "Vector Structure") (FingerIndex :type "ETouchIndex Enum"))
  (bind _returnvalue (`GameplayStatics.GetPlayerPawn` 0))
  (:`Pressed`
    (set `self.isTouchMove` false)
    (bind _output_get (set `self.StartPos` Location))
    (set `self.PrePos` _output_get))
  (:`Moved`
    (if (>= (`KismetMathLibrary.VSize` (- Location (`self.StartPos`))) (`self.Sensitivity`))
      (set `self.isTouchMove` true)
      (`self.K2_SetActorLocation` _returnvalue (+ (`self.K2_GetActorLocation` _returnvalue) (* (`KismetMathLibrary.GreaterGreater_VectorRotator` (- (`self.PrePos`) Location) (struct :`Yaw` 90.0)) (`self.Power`))) false false)
      (set `self.PrePos` Location))))

(fn `UserConstructionScript`)