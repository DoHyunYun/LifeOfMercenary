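; Battle mercenary character Blueprint that shows the battle HUD, handles touch camera yaw and release-to-unblock, and manages melee combat.
; An AttackBox on the right-hand socket deals damage on overlap, disarming after each hit.
; Incoming damage sets the Damage state and uses dot products to pass side-hit direction to the AnimBP.
; AutoAttackTarget sphere-traces nearby objects, keeping the farthest hit (or forward fallback), then turns toward it unless FreeAction is set.
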(event `self.ReceiveBeginPlay`
  (bind _returnvalue (`|CreateWidget` "/Game/UI/Battle/UI_Battle.UI_Battle_C" null self))
  (`UserWidget.AddToViewport` _returnvalue 0)
  (bind _returnvalue_2 (`LoMFunctions.GetHUDManager`))
  (`HUDManager.AddUI` _returnvalue_2 _returnvalue "Battle")
  (`HUDManager.DrawUI` _returnvalue_2 "Battle"))

(event `self.ReceiveAnyDamage`
  (params (Damage :type "Float (single-precision)") (DamageType :type "DamageType Object Reference") (InstigatedBy :type "Controller Object Reference") (DamageCauser :type "Actor Object Reference"))
  (set `self.currentState` "Damage")
  (bind _asabp_battle_mercenary (cast `/Game/Characters/Mercenary/Animation/ABP_BattleMercenary` (`SkeletalMeshComponent.GetAnimInstance` (`self.Mesh`))))
  (bind _output_get (set `self.damageDirection` (`KismetMathLibrary.Normal` (- (`self.K2_GetActorLocation`) (`self.K2_GetActorLocation` DamageCauser)))))
  (bind _returnvalue (`KismetMathLibrary.Dot_VectorVector` _output_get (`self.GetActorRightVector`)))
  (if (>= _returnvalue 0.7)
    (set `/Game/Characters/Mercenary/Animation/ABP_BattleMercenary.Check_FB_LR` true _asabp_battle_mercenary)
    (set `/Game/Characters/Mercenary/Animation/ABP_BattleMercenary.Check_LR` 1.0 _asabp_battle_mercenary)
    (elif (<= _returnvalue -0.7)
      (set `/Game/Characters/Mercenary/Animation/ABP_BattleMercenary.Check_FB_LR` true _asabp_battle_mercenary)
      (set `/Game/Characters/Mercenary/Animation/ABP_BattleMercenary.Check_LR` -1.0 _asabp_battle_mercenary)
      (else
        (set `/Game/Characters/Mercenary/Animation/ABP_BattleMercenary.Check_FB_LR` false _asabp_battle_mercenary)
        (set `CharacterMovementComponent.MaxWalkSpeed` 200.0 (`self.CharacterMovement`))))))

(event `self.AttackBox.OnComponentBeginOverlap`
  (params (OverlappedComponent :type "PrimitiveComponent Object Reference") (OtherActor :type "Actor Object Reference") (OtherComp :type "PrimitiveComponent Object Reference") (OtherBodyIndex :type Integer) (bFromSweep :type Boolean) (SweepResult :type "HitResult Structure (by ref)"))
  (if (`self.bAttackEnable`)
    (`GameplayStatics.ApplyDamage` OtherActor 100.0 null self)
    (set `self.bAttackEnable` false)))

(event `InputTouch`
  (params (Location :type "Vector Structure") (FingerIndex :type "ETouchIndex Enum"))
  (bind _x (.x Location))
  (:`Pressed`
    (set `self.OrgTouchXPoint` _x))
  (:`Released`
    (set `self.bCameraRotEnable` true)
    (if (`|EnumEquality` (`self.currentState`) "Block")
      (`self.UnBlock`)))
  (:`Moved`
    (if (`self.bCameraRotEnable`)
      (`self.AddControllerYawInput` (/ (- (`self.OrgTouchXPoint`) _x) (`self.cameraRotSpeed`)))
      (set `self.OrgTouchXPoint` _x))))

(fn `AutoAttackTarget`
  (locals (ObjectType :type "Array of EObjectTypeQuery Enum") (MaxLength :type "Float (double-precision)") (TargetLocation :type "Vector Structure" :default (0.0 0.0 0.0)))
  (bind _returnvalue (`self.K2_GetActorLocation`))
  (bind _returnvalue_2 (`KismetMathLibrary.Normal` (- (`local.TargetLocation`) (`self.K2_GetActorLocation`))))
  (`|ExecutionSequence`
    (:`then_0`
      (bind (_outhits _returnvalue_3) (`KismetSystemLibrary.SphereTraceMultiForObjects` :`Start` _returnvalue :`End` _returnvalue :`Radius` 300.0 :`ObjectTypes` (`local.ObjectType`) :`DrawDebugType` "ForOneFrame"))
      (if _returnvalue_3
        (for _array_element _outhits
          (bind _returnvalue_4 (`self.K2_GetActorLocation` (`.HitActor` (`GameplayStatics.BreakHitResult` _array_element))))
          (bind _returnvalue_5 (`KismetMathLibrary.VSize` (- (`self.K2_GetActorLocation`) _returnvalue_4)))
          (if (>= _returnvalue_5 (`local.MaxLength`))
            (set `local.MaxLength` _returnvalue_5)
            (set `local.TargetLocation` _returnvalue_4)))
        (else
          (set `local.TargetLocation` (+ (`self.GetActorForwardVector`) (`self.K2_GetActorLocation`))))))
    (:`then_1`
      (if (not (`self.bFreeAction`))
        (`self.K2_SetActorRotation` (`KismetMathLibrary.MakeRotator` 0.0 0.0 (.yaw (`KismetMathLibrary.Conv_VectorToRotator` _returnvalue_2))))
        (set `self.worldDir` _returnvalue_2)))))

(fn `UserConstructionScript`
  (`SceneComponent.K2_AttachToComponent` (`self.AttackBox`) (`self.Mesh`) "rightHand_socket" "KeepRelative" "KeepRelative" "KeepRelative" true))