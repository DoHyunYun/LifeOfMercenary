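; BP_Wolf is a wolf monster that deals bite damage and reacts to being hit.
; The construction script attaches AttackCollision to the teeth socket on the mesh.
; When that collision begins an overlap while AttackEnable is set, it applies fixed damage to the other actor and clears the flag, limiting each enable to one hit.
; Taking any damage sets CurrentState to Damage.
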(event `self.ReceiveBeginPlay`)

(event `self.ReceiveTick`
  (params (DeltaSeconds :type "Float (single-precision)")))

(event `self.ReceiveAnyDamage`
  (params (Damage :type "Float (single-precision)") (DamageType :type "DamageType Object Reference") (InstigatedBy :type "Controller Object Reference") (DamageCauser :type "Actor Object Reference"))
  (set `self.currentState` "Damage"))

(event `self.AttackCollision.OnComponentBeginOverlap`
  (params (OverlappedComponent :type "PrimitiveComponent Object Reference") (OtherActor :type "Actor Object Reference") (OtherComp :type "PrimitiveComponent Object Reference") (OtherBodyIndex :type Integer) (bFromSweep :type Boolean) (SweepResult :type "HitResult Structure (by ref)"))
  (if (`self.bAttackEnable`)
    (`GameplayStatics.ApplyDamage` OtherActor 10.0 null self)
    (set `self.bAttackEnable` false)))

(fn `UserConstructionScript`
  (`SceneComponent.K2_AttachToComponent` (`self.AttackCollision`) (`self.Mesh`) "Socket_Teeth" "KeepRelative" "KeepRelative" "KeepRelative" true))