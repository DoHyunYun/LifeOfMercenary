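; BP_MainSceneMercenary is a modular mercenary actor in the main scene that opens a player information screen when tapped.
; The construction script slaves its body, hands, feet and bottoms meshes to the main Mesh through master pose.
; BeginPlay creates the PlayerInformation widget and registers it with the HUD manager.
; Touch release on BoxCollision shows and triggers that widget only while the main scene camera's tick is off and the HUD manager is enabled.
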(event `self.ReceiveBeginPlay`
  (bind _returnvalue (`|CreateWidget` "/Game/UI/UI_PlayerInformation.UI_PlayerInformation_C" null self))
  (bind _output_get (set `self.PlayerInformation` _returnvalue))
  (`UserWidget.AddToViewport` _output_get 0)
  (bind _returnvalue_2 (`LoMFunctions.GetHUDManager`))
  (`HUDManager.AddUI` _returnvalue_2 _output_get "PlayerInformation"))

(event `self.boxCollision.OnInputTouchEnd`
  (params (FingerIndex :type "ETouchIndex Enum" :default "Touch1") (TouchedComponent :type "PrimitiveComponent Object Reference"))
  (bind _returnvalue (`LoMFunctions.GetMainSceneCamera`))
  (if (not (`self.IsActorTickEnabled` _returnvalue))
    (bind _returnvalue_2 (`LoMFunctions.GetHUDManager`))
    (if (`HUDManager.bEnable` _returnvalue_2)
      (`HUDManager.DrawUI` _returnvalue_2 "PlayerInformation")
      (`/Game/UI/UI_PlayerInformation.OnPlayerInformationUI` (`self.PlayerInformation`)))))

(fn `UserConstructionScript`
  (`SkinnedMeshComponent.SetLeaderPoseComponent` (`self.body`) (`self.Mesh`))
  (`SkinnedMeshComponent.SetLeaderPoseComponent` (`self.hands`) (`self.Mesh`))
  (`SkinnedMeshComponent.SetLeaderPoseComponent` (`self.feets`) (`self.Mesh`))
  (`SkinnedMeshComponent.SetLeaderPoseComponent` (`self.bottoms`) (`self.Mesh`)))