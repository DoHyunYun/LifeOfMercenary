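; Touchable quest board actor for the main scene that opens the UI_Board screen through the HUD manager.
; Ending a touch on its box collision binds to the main scene camera's move-exit event.
; That event re-enables query collision when Begin is true; otherwise, if the camera has stopped ticking, it draws the UI and disables collision.
; Touch enter and leave toggle custom depth rendering on the Cube.
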(event `self.boxCollision.OnInputTouchEnd`
  (params (FingerIndex :type "ETouchIndex Enum" :default "Touch1") (TouchedComponent :type "PrimitiveComponent Object Reference"))
  (bind _returnvalue (`LoMFunctions.GetMainSceneCamera`))
  (add `LoMCamera.cameraMoveExit` _returnvalue (delegate `CameraMoveExit`)))

(event `CameraMoveExit`
  (params (_begin :type Boolean))
  (if _begin
    (`PrimitiveComponent.SetCollisionEnabled` (`self.boxCollision`) "QueryOnly")
    (else
      (bind _returnvalue (`LoMFunctions.GetMainSceneCamera`))
      (if (not (`self.IsActorTickEnabled` _returnvalue))
        (bind _returnvalue_2 (`LoMFunctions.GetHUDManager`))
        (`HUDManager.DrawUI` _returnvalue_2 "UI_Board")
        (`PrimitiveComponent.SetCollisionEnabled` (`self.boxCollision`) "NoCollision")))))

(event `self.boxCollision.OnInputTouchEnter`
  (params (FingerIndex :type "ETouchIndex Enum" :default "Touch1") (TouchedComponent :type "PrimitiveComponent Object Reference"))
  (`PrimitiveComponent.SetRenderCustomDepth` (`self.Cube`) true))

(event `self.boxCollision.OnInputTouchLeave`
  (params (FingerIndex :type "ETouchIndex Enum" :default "Touch1") (TouchedComponent :type "PrimitiveComponent Object Reference"))
  (`PrimitiveComponent.SetRenderCustomDepth` (`self.Cube`) false))

(fn `UserConstructionScript`)